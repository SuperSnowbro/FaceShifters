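; Player pawn that moves in the XZ plane between planets and spawns at the game instance's saved checkpoint.
; Each tick the GetLandingState macro selects planet movement, driven through the current planet, or custom air physics with gravity, drag and steering.
; A blocking swept hit lands the pawn and hands it to the planet.
; Jumping, burrowing through non-base planets or being launched detaches it and briefly suspends gravity.
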(event Custom|ForcedPosTick)

(event EventTick
  (params (DeltaSeconds :type Float%20%28single-precision%29))
  (bind _returnvalue (Transformation|GetActorLocation))
  (bind _currentplanet (Variables|PlanetLanding|GetCurrentPlanet))
  (bind _planetsurfacecollision (Variables|/Game/Blueprints/PlatformerLogic/Superclassi/BP_BasePlanet.BP_BasePlanet_C|GetPlanetSurfaceCollision _currentplanet))
  (bind _returnvalue_2 (Transformation|GetWorldLocation _planetsurfacecollision))
  (CallFunction|ForcedPosTick)
  (CallFunction|InputTick)
  (Utilities|GetLandingState
    (:IsOnPlanet
      (CallFunction|PlanetMovementTick)
      (Transformation|SetWorldRotation (Variables|Default|GetMesh) (Math|Rotator|CombineRotators (Math|Rotator|FindLookatRotation (Math|Vector|MakeVector (.x _returnvalue) 0.0 (.z _returnvalue)) (Math|Vector|MakeVector (.x _returnvalue_2) 0.0 (.z _returnvalue_2))) "90.000000, 0,0.000000") false false))
    (:IsOnAir
      (CallFunction|GravityTick)
      (CallFunction|AirMovementTick))))

(event EventBeginPlay
  (bind _asbp_faceshifters_gi (Utilities|Casting|CastToBP_FaceshiftersGI (Game|GetGameInstance)))
  (if (Math|Vector|NotEqual(Vector) (Variables|/Game/Blueprints/BP_FaceshiftersGI.BP_FaceshiftersGI_C|GetCheckpoint _asbp_faceshifters_gi) "0, 0, 0" 0.0001)
    (Transformation|SetActorLocation (Variables|/Game/Blueprints/BP_FaceshiftersGI.BP_FaceshiftersGI_C|GetCheckpoint _asbp_faceshifters_gi) false true)))

(event Custom|Gravity%20Tick
  (Utilities|GetLandingState
    (:IsOnAir
      (if (not (Variables|Gravity|GetIsInGravityHold))
        (Variables|Movement|SetVelocity (+ (Variables|Movement|GetVelocity) (* (Variables|Gravity|GetCurrentGravity) (* (Utilities|Time|GetWorldDeltaSeconds) (Variables|Gravity|GetGravityScale)))))))))

(event Custom|GravityHold
  (params (HoldTime :type Float%20%28single-precision%29))
  (Variables|Gravity|SetIsInGravityHold true)
  (Utilities|FlowControl|RetriggerableDelay HoldTime)
  (Variables|Gravity|SetIsInGravityHold false))

(event Custom|InputTick
  (Utilities|GetLandingState
    (:IsOnPlanet
      (Default|PlanetaryMovement (Variables|PlanetLanding|GetCurrentPlanet) (* (Input|AxisValues|GetMoveRight) (Variables|PlanetLanding|GetPlanetRunSpeedMultiplier) (Variables|Movement|GetLandInputMovingSpeed))))
    (:IsOnAir
      ;[1 1 1] WIP
      (if true
        (Variables|Input|SetInputSpeed (Math|Vector|MakeVector (+ (.x (Math|Vector|Lerp(Vector) (Variables|Input|GetInputSpeed) "0, 0, 0" (* (Utilities|Time|GetWorldDeltaSeconds) (Variables|Input|GetInputChangeSpeed)))) (* (Variables|Input|GetInputChangeSpeed) (Utilities|Time|GetWorldDeltaSeconds) (Input|AxisValues|GetMoveRight))) 0.0 (.z (Math|Vector|Lerp(Vector) (Variables|Input|GetInputSpeed) "0, 0, 0" (* (Utilities|Time|GetWorldDeltaSeconds) (Variables|Input|GetInputChangeSpeed))))))))))

(event Input|ActionEvents|InputActionJump
  (params (Key :type Key%20Structure :default "AnyKey"))
  (:Pressed
    (Utilities|GetLandingState
      (:IsOnPlanet
        (CallFunction|LeavePlanetbyJumping)))))

(event Input|ActionEvents|InputActionAnnihilatePlanet
  (params (Key :type Key%20Structure :default "AnyKey"))
  (:Pressed
    (Utilities|GetLandingState
      (:IsOnPlanet
        (if (not (Variables|/Game/Blueprints/PlatformerLogic/Superclassi/BP_BasePlanet.BP_BasePlanet_C|GetIsBase (Variables|PlanetLanding|GetCurrentPlanet)))
          (CallFunction|LeaveThroughPlanet))))))

(event Input|KeyboardEvents|L
  (params (Key :type Key%20Structure :default "AnyKey"))
  ;[1 1 1] TEST FIELD
)

(event Input|MouseEvents|MiddleMouseButton
  (params (Key :type Key%20Structure :default "AnyKey"))
  (bind _returnvalue (Transformation|GetActorLocation))
  ;[1 1 1] TEST FIELD
  (:Pressed
    (Utilities|FlowControl|FlipFlop
      (:A
        (Transformation|SetActorLocation (Math|Vector|MakeVector (.x _returnvalue) -7e+03 (.z _returnvalue)) false false))
      (:B
        (Transformation|SetActorLocation (Math|Vector|MakeVector (.x _returnvalue) 0.0 (.z _returnvalue)) false false)))))

(event Custom|GetLaunched
  (params (Direction :type Vector) (Intensity :type Float%20%28single-precision%29) (InterpolationAmount :type Float%20%28single-precision%29))
  (Utilities|GetLandingState
    (:IsOnPlanet
      (CallFunction|LeavePlanetbyLaunch))
    (:IsOnAir
      _))
  (Variables|Input|SetInputSpeed "0, 0, 0")
  (Variables|Movement|SetVelocity (Math|Vector|Lerp(Vector) (Variables|Movement|GetVelocity) (* Direction Intensity) InterpolationAmount)))

(event Custom|LeavePlanetByJumping
  (CallFunction|GravityHold 0.1)
  (Transformation|DetachFromActor "KeepWorld" "KeepWorld" "KeepWorld")
  (Variables|PlanetLanding|Set£IsOnPlanet false)
  (Variables|Movement|SetVelocity (* (Math|Vector|Normalize (- (Transformation|GetActorLocation) (Transformation|GetActorLocation (Variables|PlanetLanding|GetCurrentPlanet)))) (Variables|Movement|GetJumpSpeed)))
  (Variables|PlanetLanding|SetCurrentPlanet 0))

(event Custom|PlanetMovementTick
  (Transformation|SetActorRotation (Variables|/Script/Engine.SceneComponent|GetRelativeRotation (Variables|/Game/Blueprints/PlatformerLogic/Superclassi/BP_BasePlanet.BP_BasePlanet_C|GetPlanetRotationPivot (Variables|PlanetLanding|GetCurrentPlanet))) true))

(event Custom|LeaveThroughPlanet
  (CallFunction|GravityHold 0.2)
  (Transformation|DetachFromActor "KeepWorld" "KeepWorld" "KeepWorld")
  (Default|PlanetLeft (Variables|PlanetLanding|GetCurrentPlanet))
  (Variables|PlanetLanding|Set£IsOnPlanet false)
  (Variables|Movement|SetVelocity (* (Math|Vector|Normalize (- (Transformation|GetActorLocation (Variables|PlanetLanding|GetCurrentPlanet)) (Transformation|GetActorLocation))) (Variables|Movement|GetAnnihilationSpeed)))
  (Variables|PlanetLanding|SetCurrentPlanet 0))

(event Custom|LeavePlanetByLaunch
  (CallFunction|GravityHold 0.1)
  (Transformation|DetachFromActor "KeepWorld" "KeepWorld" "KeepWorld")
  (Variables|PlanetLanding|Set£IsOnPlanet false)
  (Variables|PlanetLanding|SetCurrentPlanet 0))

(event Custom|AirMovementTick
  (CallFunction|ApplyDrag)
  (if (Class|KismetMathLibrary|XORBoolean (>= (.x (Variables|Input|GetInputSpeed)) 0.0) (>= (.x (Variables|Movement|GetVelocity)) 0.0))
    (CallFunction|Decelerate))
  (bind _sweephitresult (Transformation|AddActorWorldOffset (Math|Vector|MakeVector (.x (+ (* (Variables|Movement|GetVelocity) (Utilities|Time|GetWorldDeltaSeconds)) (* (Variables|Input|GetInputSpeed) (* (Utilities|Time|GetWorldDeltaSeconds) (Variables|Movement|GetAirInputMovingSpeed))))) 0.0 (.z (+ (* (Variables|Movement|GetVelocity) (Utilities|Time|GetWorldDeltaSeconds)) (* (Variables|Input|GetInputSpeed) (* (Utilities|Time|GetWorldDeltaSeconds) (Variables|Movement|GetAirInputMovingSpeed)))))) true))
  (Variables|PlanetLanding|Set£IsOnPlanet (.bblockinghit _sweephitresult))
  (Utilities|GetLandingState
    (:IsOnPlanet
      (Variables|Input|SetInputSpeed "0, 0, 0")
      (Variables|Movement|SetVelocity "0, 0, 0")
      ;[1 1 1] remove this and use a handshake interface
      (bind _asbp_base_planet (Utilities|Casting|CastToBP_BasePlanet (.hitactor _sweephitresult)))
      (Default|ReceiveVisitor _asbp_base_planet self))))

(fn ConstructionScript
  (bind _returnvalue (Transformation|GetActorLocation))
  (Transformation|SetActorLocation (Math|Vector|MakeVector (.x _returnvalue) 0.0 (.z _returnvalue)) false false))

(fn GetCurrentPlanet
  (return (Variables|PlanetLanding|GetCurrentPlanet)))

(fn ApplyDrag
  (Variables|Movement|SetVelocity (Math|Vector|Lerp(Vector) (Variables|Movement|GetVelocity) "0,0.000000, 0" (* (Variables|Movement|GetDrag) (Utilities|Time|GetWorldDeltaSeconds))))
  (return))

(fn Decelerate
  ;[1 1 1] WIP
  (Variables|Movement|SetVelocity (Math|Vector|MakeVector (- (Math|Float|Lerp (.x (Variables|Movement|GetVelocity)) 0.0 (* (Utilities|Time|GetWorldDeltaSeconds) (Variables|Default|GetDecelerationLerpSpeed))) (* (Math|Float|Sign(Float) (Math|Float|Lerp (.x (Variables|Movement|GetVelocity)) 0.0 (* (Utilities|Time|GetWorldDeltaSeconds) (Variables|Default|GetDecelerationLerpSpeed)))) (Variables|Default|GetDecelerationFlatAmount) (Utilities|Time|GetWorldDeltaSeconds))) 0.0 (.z (Variables|Movement|GetVelocity)))))