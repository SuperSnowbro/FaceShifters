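; Runtime creator tool that spawns a BP_EscapingPlanet and lets the player configure it with the mouse.
; NextStep advances a step counter and mode label; Tick applies the current step: scale, detection radius, escape direction and speed, then ends creation.
; Detection and direction previews are unhidden, and construction reruns to refresh radius and direction edits.
; BuildString serializes the result as Unreal actor-export text, splicing location, scale and tuned values into a hardcoded template.
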(event EventBeginPlay)

(event Collision|EventActorBeginOverlap
  (params (OtherActor :type Actor%20Object%20Reference)))

(event EventTick
  (params (DeltaSeconds :type Float%20%28single-precision%29))
  (bind _returnvalue (Game|GetPlayerController 0))
  (bind _myplanet (Variables|Default|GetMyPlanet))
  (bind _worldlocation (Game|Player|ConvertMouseLocationToWorldSpace _returnvalue))
  (bind _returnvalue_2 (Transformation|GetActorLocation _myplanet))
  (bind (_x _y _z) (Math|Vector|BreakVector _worldlocation))
  (bind _returnvalue_3 (Math|Vector|MakeVector _x 0.0 _z))
  (bind _returnvalue_4 (- _returnvalue_2 _returnvalue_3))
  (bind _returnvalue_5 (Math|Rotator|FindLookatRotation (Math|Vector|MakeVector 0.0 0.0 0.0) _returnvalue_4))
  (switch int (Variables|Default|GetDerp)
    (:0
      (CallFunction|UpdatePlanetScale))
    (:1
      (Variables|/Game/Blueprints/PlatformerLogic/Superclassi/BP_BasePlanetDetecting.BP_BasePlanetDetecting_C|SetDetectionRadius (Variables|Default|GetMyEscapingPlanet) (* (CallFunction|GetMouseDistancefromPlanet) 1e+02))
      (Default|ConstructFunction (Variables|Default|GetMyEscapingPlanet)))
    (:2
      (Variables|/Game/Blueprints/PlatformerLogic/BP_EscapingPlanet.BP_EscapingPlanet_C|SetDirectionRotation (Variables|Default|GetMyEscapingPlanet) (Math|Float|SelectFloat (* (.pitch _returnvalue_5) -1.0) (- (.pitch _returnvalue_5) 1.8e+02) (== (.yaw _returnvalue_5) 1.8e+02)))
      (bind _output_get (Variables|/Game/Blueprints/PlatformerLogic/BP_EscapingPlanet.BP_EscapingPlanet_C|SetSpeed (Variables|Default|GetMyEscapingPlanet) (+ (* (CallFunction|GetMouseDistancefromPlanet) 7e+01) 1.5e+02)))
      (Development|PrintString (Utilities|String|Append "Speed: " (Utilities|String|ToString(Float) _output_get)))
      (Default|ConstructFunction (Variables|Default|GetMyEscapingPlanet)))
    (:3
      (CallFunction|EndCreation))))

(event EventStartCreation
  (bind _returnvalue (Game|SpawnActorfromClass "/Game/Blueprints/PlatformerLogic/BP_EscapingPlanet.BP_EscapingPlanet_C" (Math|Transform|MakeTransform (CallFunction|GetPlanetLocation) "0, 0, 0" "1,1,1") "Undefined" 0 0))
  (Variables|Default|SetMyPlanet _returnvalue)
  (bind _output_get (Variables|Default|SetMyEscapingPlanet _returnvalue))
  (Development|SetHiddeninGame (Variables|/Game/Blueprints/PlatformerLogic/Superclassi/BP_BasePlanetDetecting.BP_BasePlanetDetecting_C|GetDetectionCollision _output_get) false true))

(fn ConstructionScript
  (|CallParentFunction))

(fn NextStep
  (bind _result (Math|Integer|IncrementInt (Variables|Default|GetDerp))
    (:%20%20
      (switch int _result
        (:1
          (CallFunction|UpdateUICurrentMode "Detection Radius")
          (return false))
        (:2
          (CallFunction|UpdateUICurrentMode "Escape Direction & Speed")
          (return false))
        (:3
          (CallFunction|UpdateUICurrentMode "Placement")
          (return true))))))

(fn BuildString
  (bind _myplanet (Variables|Default|GetMyPlanet))
  (bind _myplanet_2 (Variables|Default|GetMyPlanet))
  (bind _returnvalue (Transformation|GetActorLocation _myplanet_2))
  (bind _returnvalue_2 (Transformation|GetActorScale3D _myplanet))
  (bind (_x _y _z) (Math|Vector|BreakVector _returnvalue_2))
  (bind (_x_2 _y_2 _z_2) (Math|Vector|BreakVector _returnvalue))
  (Variables|Default|SetMyStringPiece " 
      Begin Actor Class=/Game/Blueprints/PlatformerLogic/BP_EscapingPlanet.BP_EscapingPlanet_C Name=BP_EscapingPlanet_114 Archetype=/Game/Blueprints/PlatformerLogic/BP_EscapingPlanet.BP_EscapingPlanet_C'/Game/Blueprints/PlatformerLogic/BP_EscapingPlanet.Default__BP_EscapingPlanet_C' 
         Begin Object Class=/Script/Engine.ArrowComponent Name=\"DirectionPreview\" Archetype=ArrowComponent'/Game/Blueprints/PlatformerLogic/BP_EscapingPlanet.BP_EscapingPlanet_C:DirectionPreview_GEN_VARIABLE' 
         End Object 
         Begin Object Class=/Script/Engine.SceneComponent Name=\"RotationPreviewPivot\" Archetype=SceneComponent'/Game/Blueprints/PlatformerLogic/BP_EscapingPlanet.BP_EscapingPlanet_C:RotationPreviewPivot_GEN_VARIABLE' 
         End Object 
         Begin Object Class=/Script/Engine.SphereComponent Name=\"DetectionCollision\" Archetype=SphereComponent'/Game/Blueprints/PlatformerLogic/BP_EscapingPlanet.BP_EscapingPlanet_C:DetectionCollision_GEN_VARIABLE' 
            Begin Object Class=/Script/Engine.BodySetup Name=\"BodySetup_880\" 
            End Object 
         End Object 
         Begin Object Class=/Script/Engine.StaticMeshComponent Name=\"PlanetVisual\" Archetype=StaticMeshComponent'/Game/Blueprints/PlatformerLogic/BP_EscapingPlanet.BP_EscapingPlanet_C:PlanetVisual_GEN_VARIABLE' 
         End Object 
         Begin Object Class=/Script/Engine.SceneComponent Name=\"PlanetRotationPivot\" Archetype=SceneComponent'/Game/Blueprints/PlatformerLogic/BP_EscapingPlanet.BP_EscapingPlanet_C:PlanetRotationPivot_GEN_VARIABLE' 
         End Object 
         Begin Object Class=/Script/Engine.SphereComponent Name=\"PlanetSurfaceCollision\" Archetype=SphereComponent'/Game/Blueprints/PlatformerLogic/BP_EscapingPlanet.BP_EscapingPlanet_C:PlanetSurfaceCollision_GEN_VARIABLE' 
         End Object 
         Begin Object Name=\"DirectionPreview\" 
            AttachParent=RotationPreviewPivot 
            RelativeScale3D=(X=1.034000,Y=1.034000,Z=1.034000) 
            bNetAddressable=True 
            CreationMethod=SimpleConstructionScript 
            UCSModifiedProperties(0)=(MemberParent=Class'/Script/Engine.SceneComponent',MemberName=\"RelativeScale3D\") 
         End Object 
         Begin Object Name=\"RotationPreviewPivot\" 
            AttachParent=PlanetSurfaceCollision 
            RelativeRotation=(Pitch=47.248356,Yaw=0.000000,Roll=0.000000) 
            bNetAddressable=True 
            CreationMethod=SimpleConstructionScript 
            UCSModifiedProperties(0)=(MemberParent=Class'/Script/Engine.SceneComponent',MemberName=\"RelativeRotation\") 
         End Object 
         Begin Object Name=\"DetectionCollision\" 
            Begin Object Name=\"BodySetup_880\" 
               AggGeom=(SphereElems=((TM=(XPlane=(W=0.000000,X=-107120278671086069114675910963888128.000000,Y=0.000000,Z=0.000000),YPlane=(W=0.000000,X=0.000000,Y=0.000000,Z=0.000000),ZPlane=(W=0.000000,X=0.000000,Y=0.000000,Z=24659940404571970910256365568.000000),WPlane=(W=0.000000,X=24660620425345504139167137792.000000,Y=0.000000,Z=0.003610)),Radius=296.603333))) 
               CollisionTraceFlag=CTF_UseSimpleAsComplex 
            End Object 
            SphereRadius=296.603333 
            AttachParent=PlanetSurfaceCollision 
            bNetAddressable=True 
            CreationMethod=SimpleConstructionScript 
            UCSModifiedProperties(0)=(MemberParent=Class'/Script/Engine.SphereComponent',MemberName=\"SphereRadius\") 
         End Object 
         Begin Object Name=\"PlanetVisual\" 
            AttachParent=PlanetSurfaceCollision 
            bNetAddressable=True 
            CreationMethod=SimpleConstructionScript 
         End Object 
         Begin Object Name=\"PlanetRotationPivot\" 
            AttachParent=PlanetSurfaceCollision 
            bNetAddressable=True 
            CreationMethod=SimpleConstructionScript 
         End Object 
         Begin Object Name=\"PlanetSurfaceCollision\" 
            RelativeLocation=(")
  (Variables|Default|SetMyStringPiece (Utilities|String|Append (Variables|Default|GetMyStringPiece) "X=" (Utilities|String|ToString(Float) _x_2) "," "Y=" (Utilities|String|ToString(Float) _y_2) "," "Z=" (Utilities|String|ToString(Float) _z_2)))
  (Variables|Default|SetMyStringPiece (Utilities|String|Append (Variables|Default|GetMyStringPiece) ") 
            RelativeScale3D=("))
  (Variables|Default|SetMyStringPiece (Utilities|String|Append (Variables|Default|GetMyStringPiece) "X=" (Utilities|String|ToString(Float) _x) "," "Y=" (Utilities|String|ToString(Float) _y) "," "Z=" (Utilities|String|ToString(Float) _z)))
  (Variables|Default|SetMyStringPiece (Utilities|String|Append (Variables|Default|GetMyStringPiece) ") 
            bNetAddressable=True 
            CreationMethod=SimpleConstructionScript 
            UCSModifiedProperties(0)=(MemberParent=Class'/Script/Engine.SceneComponent',MemberName=\"RelativeLocation\") 
            UCSModifiedProperties(1)=(MemberParent=Class'/Script/Engine.SceneComponent',MemberName=\"RelativeScale3D\") 
         End Object 
         DirectionPreview=DirectionPreview 
         RotationPreviewPivot=RotationPreviewPivot 
         Speed="))
  (CallFunction|AppendtoMyStringPiece (Utilities|String|ToString(Float) (Variables|/Game/Blueprints/PlatformerLogic/BP_EscapingPlanet.BP_EscapingPlanet_C|GetSpeed (Variables|Default|GetMyEscapingPlanet))))
  (CallFunction|AppendtoMyStringPiece " 
         DirectionRotation=")
  (CallFunction|AppendtoMyStringPiece (Utilities|String|ToString(Float) (Variables|/Game/Blueprints/PlatformerLogic/BP_EscapingPlanet.BP_EscapingPlanet_C|GetDirectionRotation (Variables|Default|GetMyEscapingPlanet))))
  (CallFunction|AppendtoMyStringPiece " 
         DetectionCollision=DetectionCollision 
         DetectionRadius=")
  (CallFunction|AppendtoMyStringPiece (Utilities|String|ToString(Float) (Variables|/Game/Blueprints/PlatformerLogic/Superclassi/BP_BasePlanetDetecting.BP_BasePlanetDetecting_C|GetDetectionRadius (Variables|Default|GetMyEscapingPlanet))))
  (CallFunction|AppendtoMyStringPiece " 
         PlanetVisual=PlanetVisual 
         PlanetSurfaceCollision=PlanetSurfaceCollision 
         PlanetRotationPivot=PlanetRotationPivot 
         DeathTime=1.588406 
         RootComponent=PlanetSurfaceCollision 
         ActorLabel=\"BP_ExplodingPlanet\" 
      End Actor 
")
  (return (Variables|Default|GetMyStringPiece)))