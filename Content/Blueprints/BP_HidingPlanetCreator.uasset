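; In-game creation tool for BP_HidingPlanet, building on inherited planet-creator helpers.
; StartCreation spawns the planet with its detection sphere visible, then NextStep advances the UI through Scaling, Detection Radius and Placement.
; Tick scales the planet, sets detection radius from mouse distance while re-running its construct function, then ends creation.
; BuildString serializes the result as editor-style actor copy text, splicing location, scale and radius into a hardcoded template.
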(event EventBeginPlay)

(event Collision|EventActorBeginOverlap
  (params (OtherActor :type Actor%20Object%20Reference)))

(event EventTick
  (params (DeltaSeconds :type Float%20%28single-precision%29))
  (bind _myhidingplanet (Variables|Default|GetMyHidingPlanet))
  (switch int (Variables|Default|GetDerp)
    (:0
      (CallFunction|UpdatePlanetScale))
    (:1
      (Variables|/Game/Blueprints/PlatformerLogic/Superclassi/BP_BasePlanetDetecting.BP_BasePlanetDetecting_C|SetDetectionRadius _myhidingplanet (* (CallFunction|GetMouseDistancefromPlanet) 1e+02))
      (Default|ConstructFunction _myhidingplanet))
    (:2
      (CallFunction|EndCreation))))

(event EventStartCreation
  (bind _returnvalue (Game|SpawnActorfromClass "/Game/Blueprints/PlatformerLogic/BP_HidingPlanet.BP_HidingPlanet_C" (Math|Transform|MakeTransform (CallFunction|GetPlanetLocation) "0, 0, 0" "1,1,1") "Undefined" 0 0))
  (Variables|Default|SetMyPlanet _returnvalue)
  (bind _output_get (Variables|Default|SetMyHidingPlanet _returnvalue))
  (Development|SetHiddeninGame (Variables|/Game/Blueprints/PlatformerLogic/Superclassi/BP_BasePlanetDetecting.BP_BasePlanetDetecting_C|GetDetectionCollision _output_get) false true)
  (CallFunction|UpdateUICurrentMode "Scaling"))

(fn ConstructionScript
  (|CallParentFunction))

(fn NextStep
  (bind _result (Math|Integer|IncrementInt (Variables|Default|GetDerp))
    (:%20%20
      (switch int _result
        (:1
          (CallFunction|UpdateUICurrentMode "Detection Radius")
          (return false))
        (:2
          (CallFunction|UpdateUICurrentMode "Placement")
          (return true))))))

(fn BuildString
  (bind _myplanet (Variables|Default|GetMyPlanet))
  (bind _myplanet_2 (Variables|Default|GetMyPlanet))
  (bind _returnvalue (Transformation|GetActorLocation _myplanet_2))
  (bind _returnvalue_2 (Transformation|GetActorScale3D _myplanet))
  (bind (_x _y _z) (Math|Vector|BreakVector _returnvalue_2))
  (bind (_x_2 _y_2 _z_2) (Math|Vector|BreakVector _returnvalue))
  (Variables|Default|SetMyStringPiece " 
      Begin Actor Class=/Game/Blueprints/PlatformerLogic/BP_HidingPlanet.BP_HidingPlanet_C Name=BP_HidingPlanet2_102 Archetype=/Game/Blueprints/PlatformerLogic/BP_HidingPlanet.BP_HidingPlanet_C'/Game/Blueprints/PlatformerLogic/BP_HidingPlanet.Default__BP_HidingPlanet_C' 
         Begin Object Class=/Script/Engine.TimelineComponent Name=\"RevealingTimeline\" 
         End Object 
         Begin Object Class=/Script/Engine.TimelineComponent Name=\"HidingTimeline\" 
         End Object 
         Begin Object Class=/Script/Engine.SphereComponent Name=\"DetectionCollision\" Archetype=SphereComponent'/Game/Blueprints/PlatformerLogic/Superclassi/BP_BasePlanetDetecting.BP_BasePlanetDetecting_C:DetectionCollision_GEN_VARIABLE' 
            Begin Object Class=/Script/Engine.BodySetup Name=\"BodySetup_1032\" 
            End Object 
         End Object 
         Begin Object Class=/Script/Engine.StaticMeshComponent Name=\"PlanetVisual\" Archetype=StaticMeshComponent'/Game/Blueprints/PlatformerLogic/BP_HidingPlanet.BP_HidingPlanet_C:PlanetVisual_GEN_VARIABLE' 
         End Object 
         Begin Object Class=/Script/Engine.SceneComponent Name=\"PlanetRotationPivot\" Archetype=SceneComponent'/Game/Blueprints/PlatformerLogic/Superclassi/BP_BasePlanet.BP_BasePlanet_C:PlanetRotationPivot_GEN_VARIABLE' 
         End Object 
         Begin Object Class=/Script/Engine.SphereComponent Name=\"PlanetSurfaceCollision\" Archetype=SphereComponent'/Game/Blueprints/PlatformerLogic/Superclassi/BP_BasePlanetDetecting.BP_BasePlanetDetecting_C:PlanetSurfaceCollision_GEN_VARIABLE' 
         End Object 
         Begin Object Name=\"RevealingTimeline\" 
            TheTimeline=(LengthMode=TL_TimelineLength,Length=0.300000,InterpFloats=((FloatCurve=CurveFloat'/Game/Blueprints/PlatformerLogic/BP_HidingPlanet.BP_HidingPlanet_C:CurveFloat_0_1',TrackName=\"ZeroOne\",FloatPropertyName=\"RevealingTimeline_ZeroOne_19CF7428434EA4826393EB98E81CC0C7\")),TimelinePostUpdateFunc=BP_HidingPlanet2_102.RevealingTimeline__UpdateFunc,TimelineFinishedFunc=BP_HidingPlanet2_102.RevealingTimeline__FinishedFunc,PropertySetObject=BP_HidingPlanet_C'BP_HidingPlanet2_102',DirectionPropertyName=\"RevealingTimeline__Direction_19CF7428434EA4826393EB98E81CC0C7\") 
            bNetAddressable=True 
            CreationMethod=UserConstructionScript 
         End Object 
         Begin Object Name=\"HidingTimeline\" 
            TheTimeline=(LengthMode=TL_TimelineLength,Length=1.000000,InterpFloats=((FloatCurve=CurveFloat'/Game/Blueprints/PlatformerLogic/BP_HidingPlanet.BP_HidingPlanet_C:CurveFloat_0',TrackName=\"OneZero\",FloatPropertyName=\"HidingTimeline_OneZero_AA0FCE414CDD6D0F7E4416BF26D96088\")),TimelinePostUpdateFunc=BP_HidingPlanet2_102.HidingTimeline__UpdateFunc,TimelineFinishedFunc=BP_HidingPlanet2_102.HidingTimeline__FinishedFunc,PropertySetObject=BP_HidingPlanet_C'BP_HidingPlanet2_102',DirectionPropertyName=\"HidingTimeline__Direction_AA0FCE414CDD6D0F7E4416BF26D96088\") 
            bNetAddressable=True 
            CreationMethod=UserConstructionScript 
         End Object 
         Begin Object Name=\"DetectionCollision\" 
            Begin Object Name=\"BodySetup_1032\" 
               AggGeom=(SphereElems=((TM=(XPlane=(W=0.000000,X=-529635237276447499955474530304.000000,Y=0.000000,Z=0.000000),YPlane=(W=0.000000,X=0.000000,Y=0.000000,Z=0.000000),ZPlane=(W=0.000000,X=0.000000,Y=0.000000,Z=24645697747259636060291858432.000000),WPlane=(W=0.000000,X=24643959916393940030853218304.000000,Y=0.000000,Z=0.003610)),Radius=770.416931))) 
               CollisionTraceFlag=CTF_UseSimpleAsComplex 
            End Object 
            SphereRadius=770.416931 
            AttachParent=PlanetSurfaceCollision 
            bNetAddressable=True 
            CreationMethod=SimpleConstructionScript 
            UCSModifiedProperties(0)=(MemberParent=Class'/Script/Engine.SphereComponent',MemberName=\"SphereRadius\") 
         End Object 
         Begin Object Name=\"PlanetVisual\" 
            AttachParent=PlanetSurfaceCollision 
            bNetAddressable=True 
            CreationMethod=SimpleConstructionScript 
         End Object 
         Begin Object Name=\"PlanetRotationPivot\" 
            AttachParent=PlanetSurfaceCollision 
            bNetAddressable=True 
            CreationMethod=SimpleConstructionScript 
         End Object 
         Begin Object Name=\"PlanetSurfaceCollision\" 
            RelativeLocation=(")
  (Variables|Default|SetMyStringPiece (Utilities|String|Append (Variables|Default|GetMyStringPiece) "X=" (Utilities|String|ToString(Float) _x_2) "," "Y=" (Utilities|String|ToString(Float) _y_2) "," "Z=" (Utilities|String|ToString(Float) _z_2)))
  (Variables|Default|SetMyStringPiece (Utilities|String|Append (Variables|Default|GetMyStringPiece) ") 
            RelativeScale3D=("))
  (Variables|Default|SetMyStringPiece (Utilities|String|Append (Variables|Default|GetMyStringPiece) "X=" (Utilities|String|ToString(Float) _x) "," "Y=" (Utilities|String|ToString(Float) _y) "," "Z=" (Utilities|String|ToString(Float) _z)))
  (Variables|Default|SetMyStringPiece (Utilities|String|Append (Variables|Default|GetMyStringPiece) ") 
            bNetAddressable=True 
            CreationMethod=SimpleConstructionScript 
            UCSModifiedProperties(0)=(MemberParent=Class'/Script/Engine.SceneComponent',MemberName=\"RelativeLocation\") 
            UCSModifiedProperties(1)=(MemberParent=Class'/Script/Engine.SceneComponent',MemberName=\"RelativeScale3D\") 
         End Object 
         RevealingTimeline=TimelineComponent'RevealingTimeline' 
         HidingTimeline=TimelineComponent'HidingTimeline' 
         DetectionCollision=DetectionCollision 
         DetectionRadius="))
  (CallFunction|AppendtoMyStringPiece (Utilities|String|ToString(Float) (Variables|/Game/Blueprints/PlatformerLogic/Superclassi/BP_BasePlanetDetecting.BP_BasePlanetDetecting_C|GetDetectionRadius (Variables|Default|GetMyHidingPlanet))))
  (CallFunction|AppendtoMyStringPiece " 
         PlanetVisual=PlanetVisual 
         PlanetSurfaceCollision=PlanetSurfaceCollision 
         PlanetRotationPivot=PlanetRotationPivot 
         RootComponent=PlanetSurfaceCollision 
         ActorLabel=\"BP_HidingPlanet2\" 
      End Actor 
")
  (return (Variables|Default|GetMyStringPiece)))