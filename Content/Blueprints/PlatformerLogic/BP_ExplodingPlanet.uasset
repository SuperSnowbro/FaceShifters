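; BP_ExplodingPlanet is a planet that explodes after a timed buildup once it detects the character or receives a visitor.
; Either trigger reveals a preview volume, which a DeathTime-scaled timeline grows to ExplosionRadius; the construction script shows that full size in editor.
; When the timeline finishes, it launches any overlapping player pawn away from its center, then destroys itself.
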(event EventBeginPlay
  (Components|Timeline|SetPlayRate (Variables|Default|GetExplosionBuildup) (/ 1.0 (Variables|Default|GetDeathTime))))

(event EventDie
  (bind _explosionpreview (Variables|Default|GetExplosionPreview))
  (bind _overlappingactors (Collision|GetOverlappingActors _explosionpreview "/Game/Blueprints/Pawns/BP_PlayerPawn.BP_PlayerPawn_C" :!class /Script/Engine.PrimitiveComponent))
  (bind _item (Utilities|Array|Get(acopy) _overlappingactors))
  (Utilities|FlowControl|DoOnce false
    (:Completed
      (Utilities|FlowControl|Sequence
        (:then_0
          (if (Utilities|Array|IsValidIndex _overlappingactors)
            (bind _asbp_player_pawn (Utilities|Casting|CastToBP_PlayerPawn _item))
            (Default|GetLaunched _asbp_player_pawn (Math|Vector|Normalize (- (Transformation|GetActorLocation _item) (Transformation|GetActorLocation))) (Variables|Default|GetExplosionIntensity) (Variables|Default|GetStrengthInterpAmout))))
        (:then_1
          (Actor|DestroyActor))))))

(event EventCharacterDetected
  (|CallParentFunction)
  (Utilities|FlowControl|DoOnce false
    (:Completed
      (Development|SetHiddeninGame (Variables|Default|GetExplosionPreview) false true)
      (bind _zeroone (Timeline|ExplosionBuildup Play)
        (:Update
          (Transformation|SetWorldScale3D (Variables|Default|GetExplosionPreview) (Math|Conversions|ToVector(Float) (* _zeroone (Variables|Default|GetExplosionRadius)))))
        (:Finished
          (CallFunction|Die))))))

(event EventVisitor
  (params (Visitor :type BP%20Player%20Pawn%20Object%20Reference))
  (|CallParentFunction Visitor)
  (Utilities|FlowControl|DoOnce false
    (:Completed
      (Development|SetHiddeninGame (Variables|Default|GetExplosionPreview) false true)
      (bind _zeroone (Timeline|ExplosionBuildup Play)
        (:Update
          (Transformation|SetWorldScale3D (Variables|Default|GetExplosionPreview) (Math|Conversions|ToVector(Float) (* _zeroone (Variables|Default|GetExplosionRadius)))))
        (:Finished
          (CallFunction|Die))))))

(fn ConstructionScript
  (|CallParentFunction)
  (Transformation|SetWorldScale3D (Variables|Default|GetExplosionPreview) (Math|Conversions|ToVector(Float) (Variables|Default|GetExplosionRadius))))