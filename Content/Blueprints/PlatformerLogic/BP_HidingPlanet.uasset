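; Planet actor for the platformer that hides or reveals its visual in response to character detection and visitors, extending a parent's events.
; BeginPlay creates a dynamic material instance on PlanetVisual, whose "alpha" parameter is driven by HidingTimeline.
; CharacterDetected plays the timeline forward, while Visitor sets its play rate to fourfold and reverses it.
; The faster rate is never reset, so it carries into later forward plays.
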(event EventBeginPlay
  (bind _returnvalue (Rendering|Material|CreateDynamicMaterialInstance (Variables|Default|GetPlanetVisual) 0 "/Game/Assets/Materials/MI_HidingPlanet.MI_HidingPlanet" :!class /Script/Engine.PrimitiveComponent))
  (Variables|Default|SetMaterialInstanceHurray _returnvalue))

(event Collision|EventActorBeginOverlap
  (params (OtherActor :type Actor%20Object%20Reference)))

(event EventTick
  (params (DeltaSeconds :type Float%20%28single-precision%29)))

(event EventCharacterDetected
  (|CallParentFunction)
  (bind _onezero (Timeline|HidingTimeline Play)
    (:Update
      (Rendering|Material|SetScalarParameterValue (Variables|Default|GetMaterialInstanceHurray) "alpha" _onezero :!class /Script/Engine.MaterialInstanceDynamic))))

(event EventVisitor
  (params (Visitor :type BP%20Player%20Pawn%20Object%20Reference))
  (|CallParentFunction Visitor)
  (Components|Timeline|SetPlayRate (Variables|Default|GetHidingTimeline) 4.0)
  (bind _onezero (Timeline|HidingTimeline Reverse)
    (:Update
      (Rendering|Material|SetScalarParameterValue (Variables|Default|GetMaterialInstanceHurray) "alpha" _onezero :!class /Script/Engine.MaterialInstanceDynamic))))

(fn ConstructionScript
  (|CallParentFunction))