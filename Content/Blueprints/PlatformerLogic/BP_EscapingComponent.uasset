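; BP_EscapingComponent is a component that moves a target actor steadily along a set direction, as its name suggests for escape movement in platformer logic.
; On BeginPlay, it defaults Target to its owning actor when none is valid.
; Each Tick, it offsets Target in local space by Direction times Speed and delta time, without sweeping for collision.
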(event EventBeginPlay
  (Utilities|IsValid (Variables|Default|GetTarget)
    (:Is%20Not%20Valid
      (Variables|Default|SetTarget (Components|GetOwner)))))

(event EventTick
  (params (DeltaSeconds :type Float%20%28single-precision%29))
  (Transformation|AddActorLocalOffset (Variables|Default|GetTarget) (* (Variables|Default|Getdirection) (* (Variables|Default|Getspeed) DeltaSeconds)) false false))