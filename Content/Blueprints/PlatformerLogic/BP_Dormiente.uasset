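; BP_Dormiente is a platformer actor with a paper sprite that dies when its CharacteronFloor event fires.
; On BeginPlay it copies MyDeathTime into DeathTime.
; The event swaps in a falling-box sprite, plays a random SuoniMorte sound and calls Die.
; It then layers a quieter random DeathSounds clip, guarding only that second array against being empty.
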(event EventBeginPlay
  (Variables|Default|SetDeathTime (Variables|Default|GetMyDeathTime)))

(event EventActorBeginOverlap
  (params (OtherActor :type Actor%20Object%20Reference)))

(event EventTick
  (params (DeltaSeconds :type Float%20%28single-precision%29)))

(event EventCharacteronFloor
  (bind _suoni_morte (Variables|Default|GetSuoni%20Morte))
  (bind _deathsounds (Variables|Default|GetDeathSounds))
  (Utilities|FlowControl|Sequence
    (:then_0
      (Rendering|Components|Sprite|SetSprite (Variables|Default|GetPaperSprite) "/Game/immagini/New-Sprites/BoxFalling_fall_Sprite.BoxFalling_fall_Sprite")
      (Audio|PlaySound2D (Utilities|Array|Get(acopy) _suoni_morte (Math|Random|RandomInteger (Utilities|Array|Length _suoni_morte))))
      (CallFunction|Die))
    (:then_1
      (if (not (== (Utilities|Array|Length _deathsounds) 0))
        (Audio|PlaySound2D (Utilities|Array|Get(acopy) _deathsounds (Math|Random|RandomInteger (Utilities|Array|Length _deathsounds))) 0.2)))))

(fn ConstructionScript
  (|CallParentFunction))