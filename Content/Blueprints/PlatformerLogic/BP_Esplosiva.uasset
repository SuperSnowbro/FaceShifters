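; BP_Esplosiva is an exploding platformer actor that detonates when a character enters its circular trigger.
; BeginPlay overrides the inherited DeathTime with its own value, which serves as the fuse after the trigger calls Die.
; During the fuse it shows a grunt sprite and plays a random charge sound.
; It then spawns a scaled BP_Esplosione carrying Power, switches to a scream sprite with a random blast sound, and destroys itself shortly afterwards.
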(event EventBeginPlay
  (|CallParentFunction)
  (Variables|Default|SetDeathTime (Variables|Default|GetMyDeathTime)))

(event EventCharacterEnterCircularTrigger
  (bind _explosionchargesounds (Variables|Default|GetExplosionChargeSounds))
  (bind _explosionsounds (Variables|Default|GetExplosionSounds))
  (Audio|PlaySound2D (Utilities|Array|Get(acopy) _explosionchargesounds (Math|Random|RandomInteger (Utilities|Array|Length _explosionchargesounds))) 0.2)
  (CallFunction|Die)
  (Rendering|Components|Sprite|SetSprite (Variables|Default|GetPaperSprite) "/Game/immagini/New-Sprites/Explodo_grunt_Sprite.Explodo_grunt_Sprite")
  (Utilities|FlowControl|Delay (Variables|Default|GetDeathTime))
  (Game|SpawnActorfromClass "/Game/Blueprints/PlatformerLogic/BP_Esplosione.BP_Esplosione_C" (Math|Transform|MakeTransform (Transformation|GetActorLocation) "0, 0, 0" (Variables|Default|GetExplosionScale)) "AlwaysSpawn" 0 (Variables|Default|GetPower) 0)
  (Audio|PlaySound2D (Utilities|Array|Get(acopy) _explosionsounds (Math|Random|RandomInteger (Utilities|Array|Length _explosionsounds))) 0.5)
  (Rendering|Components|Sprite|SetSprite (Variables|Default|GetPaperSprite) "/Game/immagini/New-Sprites/Explodo_scream_Sprite.Explodo_scream_Sprite")
  (Utilities|FlowControl|Delay 0.2)
  (Actor|DestroyActor))

(fn ConstructionScript
  (|CallParentFunction))