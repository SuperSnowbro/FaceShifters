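; Platformer checkpoint actor that saves a new checkpoint when BP_Tumy overlaps its box.
; The overlap compares the SpawnPoint's world location with the checkpoint stored in BP_FaceshiftersGI, using a small tolerance.
; If they differ, it plays a sound and passes the location to the game instance through NewCheckpoint.
; The construction script snaps the actor to X = 0, keeping its Y and Z.
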(event OnComponentBeginOverlap(Box)
  (params (OverlappedComponent :type Primitive%20Component%20Object%20Reference) (OtherActor :type Actor%20Object%20Reference) (OtherComp :type Primitive%20Component%20Object%20Reference) (OtherBodyIndex :type Integer) (bFromSweep :type Boolean) (SweepResult :type Hit%20Result%20Structure%20%28by%20ref%29))
  (Utilities|Casting|CastToBP_Tumy OtherActor)
  (bind _asbp_faceshifters_gi (Utilities|Casting|CastToBP_FaceshiftersGI (Game|GetGameInstance)))
  (if (Math|Vector|NotEqual(Vector) (Variables|/Game/Blueprints/BP_FaceshiftersGI.BP_FaceshiftersGI_C|GetCheckpoint _asbp_faceshifters_gi) (Transformation|GetWorldLocation (Variables|Default|GetSpawnPoint)) 0.1)
    (Audio|PlaySound2D (Variables|Default|GetSound) (Variables|Default|GetVolume))
    (bind _asbp_faceshifters_gi_2 (Utilities|Casting|CastToBP_FaceshiftersGI (Game|GetGameInstance)))
    (Default|NewCheckpoint _asbp_faceshifters_gi_2 (Transformation|GetWorldLocation (Variables|Default|GetSpawnPoint)))))

(event EventBeginPlay)

(event Collision|EventActorBeginOverlap
  (params (OtherActor :type Actor%20Object%20Reference)))

(event EventTick
  (params (DeltaSeconds :type Float%20%28single-precision%29)))

(fn ConstructionScript
  (bind _returnvalue (Transformation|GetActorLocation))
  (Transformation|SetActorLocation (Math|Vector|MakeVector 0.0 (.y _returnvalue) (.z _returnvalue)) false false))