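; BP_Fuggiasca is a 2D platformer runaway box that flees along a set direction when a character enters its circular trigger.
; Trigger events toggle Tick movement and running or neutral sprites, with a random flee sound on entry and an option to keep moving after exit.
; The CharacteronFloor event calls Die, shows the dead sprite, stops movement and audio, plays a random death sound and blocks further flight.
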(event EventBeginPlay
  (Variables|Default|SetDeathTime (Variables|Default|GetMyDeathTime)))

(event EventActorBeginOverlap
  (params (OtherActor :type Actor%20Object%20Reference)))

(event EventTick
  (params (DeltaSeconds :type Float%20%28single-precision%29))
  (Transformation|AddActorLocalOffset (* (Variables|Default|Getdirection) (* (Variables|Default|Getspeed) DeltaSeconds)) false false))

(event EventCharacterEnterCircularTrigger
  (bind _suonifuga (Variables|Default|GetSuoniFuga))
  (if (not (Variables|Default|Getis%20dying))
    (Rendering|Components|Sprite|SetSprite (Variables|Default|GetPaperSprite) "/Game/immagini/Sprite/BoxRunn_running_Sprite.BoxRunn_running_Sprite")
    (Actor|Tick|SetActorTickEnabled true)
    (Audio|Components|Audio|SetSound (Variables|Default|GetAudio) (Utilities|Array|Get(acopy) _suonifuga (Math|Random|RandomInteger (Utilities|Array|Length _suonifuga))))
    (Audio|Components|Audio|Play (Variables|Default|GetAudio) 0.0)
    (Utilities|FlowControl|Delay 4.0)))

(event EventCharacteronFloor
  (bind _suonimorte (Variables|Default|GetSuoniMorte))
  (Utilities|FlowControl|Sequence
    (:then_0
      (CallFunction|Die))
    (:then_1
      (Rendering|Components|Sprite|SetSprite (Variables|Default|GetPaperSprite) "/Game/immagini/Sprite/BoxRunn_dead_Sprite.BoxRunn_dead_Sprite"))
    (:then_2
      (Actor|Tick|SetActorTickEnabled false))
    (:then_3
      (Audio|Components|Audio|Stop (Variables|Default|GetAudio)))
    (:then_4
      (Audio|PlaySound2D (Utilities|Array|Get(acopy) _suonimorte (Math|Random|RandomInteger (Utilities|Array|Length _suonimorte))) 0.5))
    (:then_5
      (Variables|Default|Setis%20dying true))))

(event EventCharacterLeftCircularTrigger
  (if (not (Variables|Default|Getrimane%20in%20movimento))
    (Rendering|Components|Sprite|SetSprite (Variables|Default|GetPaperSprite) "/Game/immagini/Sprite/BoxRunn_neutral_Sprite.BoxRunn_neutral_Sprite")
    (Actor|Tick|SetActorTickEnabled false)))

(fn ConstructionScript
  (|CallParentFunction))