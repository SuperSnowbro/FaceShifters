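; BP_Spaventata is a scared, crying Paper2D platformer actor that flees and dies some time after a character lands on it.
; CharacteronFloor swaps the sprite, enables Tick and plays a random fright sound, then waits DeathTime before a random death sound and the inherited Die.
; Tick moves it along Direction at Speed without sweeping; BeginPlay sets DeathTime from MyDeathTime.
; An older timeline-based movement remains disconnected.
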(event EventBeginPlay
  (Variables|Default|SetDeathTime (Variables|Default|GetMyDeathTime)))

(event Collision|EventActorBeginOverlap
  (params (OtherActor :type Actor%20Object%20Reference)))

(event EventTick
  (params (DeltaSeconds :type Float%20%28single-precision%29))
  (Transformation|AddActorWorldOffset (* (Variables|Default|GetDirection) (* DeltaSeconds (Variables|Default|GetSpeed)))))

(event EventCharacteronFloor
  (bind _suoni_spavento (Variables|Default|Getsuoni_spavento))
  (bind _suoni_morte (Variables|Default|Getsuoni%20morte))
  (Rendering|Components|Sprite|SetSprite (Variables|Default|GetPaperSprite) "/Game/immagini/New-Sprites/BoxDepri_crying_Sprite.BoxDepri_crying_Sprite")
  (Actor|Tick|SetActorTickEnabled true)
  (Audio|PlaySound2D (Utilities|Array|Get(acopy) _suoni_spavento (Math|Random|RandomInteger (Utilities|Array|Length _suoni_spavento))) 0.4)
  (Utilities|FlowControl|Delay (Variables|Default|GetDeathTime))
  (Audio|PlaySound2D (Utilities|Array|Get(acopy) _suoni_morte (Math|Random|RandomInteger (Utilities|Array|Length _suoni_morte))))
  (CallFunction|Die))

(fn ConstructionScript
  (|CallParentFunction))