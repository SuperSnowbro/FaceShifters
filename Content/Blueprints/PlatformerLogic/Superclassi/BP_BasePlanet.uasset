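; Base class for platformer planets that a visitor lands on and moves around.
; An arriving visitor attaches to a rotation pivot, which axis input pitches at a rate partly normalized by planet scale.
; Non-base planets die after a delay by adding a faller component, and leaving disables surface collision.
; The construction script snaps each planet's Y position to its row.
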(event Custom|ReceiveVisitor
  (params (Visitor :type BP%20Player%20Pawn%20Object%20Reference))
  (bind _output_get (Variables|Default|SetVisitor Visitor))
  (Variables|/Game/Blueprints/Pawns/BP_PlayerPawn.BP_PlayerPawn_C|SetCurrentPlanet _output_get self)
  (Transformation|AttachComponentToComponent (Variables|Default|GetVisitor) (Variables|Default|GetPlanetRotationPivot) "None" "KeepWorld" "KeepWorld" "KeepWorld" true)
  (if (not (Variables|Default|GetIsBase))
    (Utilities|FlowControl|Delay (Variables|Default|GetDeathTime))
    (CallFunction|Die)))

(event Custom|PlanetLeft
  (Collision|SetCollisionEnabled (Variables|Default|GetPlanetSurfaceCollision) "NoCollision"))

(event Custom|Die
  (AddComponent|AddBPFallerComponent))

(event Custom|PlanetaryMovement
  (params (AxisInput :type Float%20%28single-precision%29))
  (Variables|Default|SetDesiredRotation (Math|Rotator|MakeRotator 0.0 (+ (.pitch (Variables|Default|GetDesiredRotation)) (* (Math|Float|Lerp (/ AxisInput (.x (Transformation|GetActorScale3D))) AxisInput 0.2) (Utilities|Time|GetWorldDeltaSeconds))) 0.0))
  (Transformation|SetWorldRotation (Variables|Default|GetPlanetRotationPivot) (Variables|Default|GetDesiredRotation) false false))

(fn ConstructionScript
  (CallFunction|ConstructFunction))

(fn ConstructFunction
  (bind _returnvalue (Transformation|GetActorLocation))
  (Transformation|SetActorLocation (Math|Vector|MakeVector (.x _returnvalue) (* (Variables|Default|GetMyRow) (Variables|Default|GetRowDistance)) (.z _returnvalue)) false true)
  (return true))