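; Base platform actor for the platformer, with overridable events for BP_Tumy landing on or leaving it.
; The first floor-collider overlap fires the landing events, passing Tumy's velocity for animation, then destroys the collider.
; Die tints the sprite to a dead color over DeathTime, then adds a BPFaller component; older fall, bob and fade logic is disconnected.
; Construction pins the actor to X=0 and derives sprite width from actor Y scale.
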(event OnComponentBeginOverlap(PavimentoCollider)
  (params (OverlappedComponent :type Primitive%20Component%20Object%20Reference) (OtherActor :type Actor%20Object%20Reference) (OtherComp :type Primitive%20Component%20Object%20Reference) (OtherBodyIndex :type Integer) (bFromSweep :type Boolean) (SweepResult :type Hit%20Result%20Structure%20%28by%20ref%29))
  (bind _asbp_tumy (Utilities|Casting|CastToBP_Tumy OtherActor))
  (CallFunction|CharacteronFloor)
  (CallFunction|CharacteronFloorAnimation (Variables|/Script/Engine.MovementComponent|GetVelocity (Pawn|GetMovementComponent _asbp_tumy)))
  (Components|DestroyComponent (Variables|Default|GetPavimentoCollider)))

(event OnComponentEndOverlap(PavimentoCollider)
  (params (OverlappedComponent :type Primitive%20Component%20Object%20Reference) (OtherActor :type Actor%20Object%20Reference) (OtherComp :type Primitive%20Component%20Object%20Reference) (OtherBodyIndex :type Integer))
  (Utilities|Casting|CastToBP_Tumy OtherActor)
  (CallFunction|CharacterLeftFloor))

(event Custom|CharacterOnFloorAnimation
  (params (Velocity :type Vector)))

(event Custom|Die
  (Components|Timeline|SetPlayRate (Variables|Default|GetDeath) (/ 1.0 (Variables|Default|GetDeathTime)))
  (bind _zeroone (Timeline|Death Play)
    (:Update
      (Sprite|SetSpriteColor (Variables|Default|GetPaperSprite) (Math|Color|Lerp(LinearColor) (Variables|Default|GetStartColor) (Variables|Default|GetDeadColor) _zeroone)))
    (:Finished
      (AddComponent|AddBPFallerComponent))))

(event Custom|Character%20On%20Floor)

(event Custom|Character%20Left%20Floor)

(event EventActorBeginOverlap
  (params (OtherActor :type Actor%20Object%20Reference)))

(event EventTick
  (params (DeltaSeconds :type Float%20%28single-precision%29)))

(event EventBeginPlay)

(fn ConstructionScript
  (bind _returnvalue (Transformation|GetActorScale3D))
  (bind _returnvalue_2 (Transformation|GetActorLocation))
  (bind _papersprite (Variables|Default|GetPaperSprite))
  (Transformation|SetActorLocation (Math|Vector|MakeVector 0.0 (.y _returnvalue_2) (.z _returnvalue_2)) false false)
  (Transformation|SetRelativeScale3D _papersprite (Math|Vector|MakeVector (* (.x (* (Math|Vector|MakeVector (.y _returnvalue) (.y _returnvalue) (.z _returnvalue)) 0.14)) (Variables|Default|GetxSpriteScaleMultiplier)) 1.0 (.z (Variables|/Script/Engine.SceneComponent|GetRelativeScale3D _papersprite)))))