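; Base planet-detection Blueprint in the platformer logic that senses when a player-tagged actor enters or leaves a detection sphere.
; Overlap begin and end on DetectionCollision fire CharacterDetected and CharacterLeftDetection, both left empty as hooks for child classes.
; The construction script runs the parent's, then divides DetectionRadius by the actor's X scale, keeping the sphere's world-space radius independent of uniform scaling.
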(event OnComponentEndOverlap(DetectionCollision)
  (params (OverlappedComponent :type Primitive%20Component%20Object%20Reference) (OtherActor :type Actor%20Object%20Reference) (OtherComp :type Primitive%20Component%20Object%20Reference) (OtherBodyIndex :type Integer))
  (if (Actor|ActorHasTag OtherActor "player")
    (CallFunction|CharacterLeftDetection)))

(event OnComponentBeginOverlap(DetectionCollision)
  (params (OverlappedComponent :type Primitive%20Component%20Object%20Reference) (OtherActor :type Actor%20Object%20Reference) (OtherComp :type Primitive%20Component%20Object%20Reference) (OtherBodyIndex :type Integer) (bFromSweep :type Boolean) (SweepResult :type Hit%20Result%20Structure%20%28by%20ref%29))
  (if (Actor|ActorHasTag OtherActor "player")
    (CallFunction|CharacterDetected)))

(event Custom|CharacterLeftDetection)

(event Custom|CharacterDetected)

(fn ConstructionScript
  (|CallParentFunction)
  (Components|Sphere|SetSphereRadius (Variables|Default|GetDetectionCollision) (/ (Variables|Default|GetDetectionRadius) (.x (Transformation|GetActorScale3D))) false))