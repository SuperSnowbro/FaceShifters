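; BP_FallerComponent is a component that moves its owning actor along the world Z axis, as a faller in the platformer logic.
; Each tick it offsets the owner by Speed scaled by delta time, without physics simulation.
; BeginPlay waits StartAugmentDelay, then sets IsAugmenting, after which Tick grows Speed by Augment per second for a linear acceleration.
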(event EventBeginPlay
  (Utilities|FlowControl|Delay (Variables|Default|GetStartAugmentDelay))
  (Variables|Default|SetisAugmenting true))

(event EventTick
  (params (DeltaSeconds :type Float%20%28single-precision%29))
  (Transformation|AddActorWorldOffset (Components|GetOwner) (Math|Vector|MakeVector 0.0 0.0 (* DeltaSeconds (Variables|Default|GetSpeed))))
  (if (Variables|Default|GetisAugmenting)
    (Variables|Default|SetSpeed (+ (* DeltaSeconds (Variables|Default|GetAugment)) (Variables|Default|GetSpeed)))))