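; BP_EscapingPlanet is a planet Blueprint for the platformer that flees once it detects the character.
; On the first detection it adds a BPEscaping component, passing its Speed and the forward vector of a DirectionPreview component.
; Its construct function extends the parent's, rotating the preview pivot to DirectionRotation and scaling the preview with Speed, so escape direction and speed are visible.
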(event EventBeginPlay)

(event Collision|EventActorBeginOverlap
  (params (OtherActor :type Actor%20Object%20Reference)))

(event EventTick
  (params (DeltaSeconds :type Float%20%28single-precision%29)))

(event EventCharacterDetected
  (|CallParentFunction)
  (Utilities|FlowControl|DoOnce false
    (:Completed
      (AddComponent|AddBPEscapingComponent 0 (Variables|Default|GetSpeed) (Math|Vector|GetForwardVector (Variables|Default|GetDirectionPreview))))))

(fn ConstructionScript
  (|CallParentFunction))

(fn ConstructFunction
  (|CallParentFunction)
  (Transformation|SetWorldRotation (Variables|Default|GetRotationPreviewPivot) (Math|Rotator|MakeRotator 0.0 (Variables|Default|GetDirectionRotation) 0.0) false true)
  (Transformation|SetWorldScale3D (Variables|Default|GetDirectionPreview) (Math|Conversions|ToVector(Float) (* (Variables|Default|GetSpeed) 0.004)))
  (return true))