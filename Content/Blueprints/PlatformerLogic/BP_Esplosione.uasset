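; BP_Esplosione is a short-lived explosion actor that knocks BP_Tumy characters away and destroys itself 0.2 seconds after BeginPlay.
; On actor overlap, it launches the overlapping BP_Tumy along the direction from its center to the first Tumy inside its Sphere, scaled by Power and overriding current velocity.
; A check for Tumys already inside the Sphere is left unconnected and never runs.
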(event EventBeginPlay
  (Utilities|FlowControl|Delay 0.2)
  (Actor|DestroyActor))

(event EventActorBeginOverlap
  (params (OtherActor :type Actor%20Object%20Reference))
  (bind _asbp_tumy (Utilities|Casting|CastToBP_Tumy OtherActor))
  (Character|LaunchCharacter _asbp_tumy (* (Math|Vector|Normalize (- (Transformation|GetActorLocation (Utilities|Array|Get(acopy) (Collision|GetOverlappingActors (Variables|Default|GetSphere) "/Game/Blueprints/Tumy/BP_Tumy.BP_Tumy_C" :!class /Script/Engine.PrimitiveComponent))) (Transformation|GetActorLocation))) (Variables|Default|GetPower)) true true))

(event EventTick
  (params (DeltaSeconds :type Float%20%28single-precision%29)))

(fn ConstructionScript)