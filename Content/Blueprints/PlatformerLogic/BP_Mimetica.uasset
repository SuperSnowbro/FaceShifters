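; BP_Mimetica is a camouflaging platformer entity that fades when the character enters its circular trigger and dies once the character is on the floor.
; Trigger entry swaps to a neutral sprite, plays a random sound and drives sprite alpha through the Fade timeline, rate-scaled by FadeTime.
; The floor event reverses the timeline over UnfadeTime, shows a sick sprite with a random death sound, then calls Die.
; BeginPlay sets DeathTime from MyDeathTime.
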(event EventBeginPlay
  (Variables|Default|SetDeathTime (Variables|Default|GetMyDeathTime)))

(event EventCharacteronFloor
  (bind _suoni_morte (Variables|Default|Getsuoni%20morte))
  (Utilities|FlowControl|Sequence
    (:then_0
      (Components|Timeline|SetPlayRate (Variables|Default|GetFade) (/ 1.0 (Variables|Default|GetUnfadeTime)))
      (bind _opacity (Timeline|Fade Reverse)
        (:Update
          (Sprite|SetSpriteColor (Variables|Default|GetPaperSprite) (Utilities|Struct|MakeLinearColor 1.0 1.0 1.0 _opacity)))))
    (:then_1
      (Utilities|FlowControl|Delay (Variables|Default|GetUnfadeTime))
      (CallFunction|Die))
    (:then_2
      (Rendering|Components|Sprite|SetSprite (Variables|Default|GetPaperSprite) "/Game/immagini/New-Sprites/Fade_sick_Sprite.Fade_sick_Sprite")
      (Audio|PlaySound2D (Utilities|Array|Get(acopy) _suoni_morte (Math|Random|RandomInteger (Utilities|Array|Length _suoni_morte))) 0.25))))

(event Collision|EventActorBeginOverlap
  (params (OtherActor :type Actor%20Object%20Reference)))

(event EventTick
  (params (DeltaSeconds :type Float%20%28single-precision%29)))

(event EventCharacterEnterCircularTrigger
  (bind _suoni_fade (Variables|Default|Getsuoni%20fade))
  (Rendering|Components|Sprite|SetSprite (Variables|Default|GetPaperSprite) "/Game/immagini/New-Sprites/Fade_neutral_Sprite.Fade_neutral_Sprite")
  (Utilities|FlowControl|Sequence
    (:then_0
      (Audio|PlaySound2D (Utilities|Array|Get(acopy) _suoni_fade (Math|Random|RandomInteger (Utilities|Array|Length _suoni_fade))) 0.25)
      (Utilities|FlowControl|Delay 3.0))
    (:then_1
      (Components|Timeline|SetPlayRate (Variables|Default|GetFade) (/ 1.0 (Variables|Default|GetFadeTime)))
      (bind _opacity (Timeline|Fade Play)
        (:Update
          (Sprite|SetSpriteColor (Variables|Default|GetPaperSprite) (Utilities|Struct|MakeLinearColor 1.0 1.0 1.0 _opacity)))))))

(fn ConstructionScript
  (|CallParentFunction))