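; Level-design tool actor that takes over input from the LevelDesignHelper to create a BP_BasePlanet at the mouse on the Y=0 plane.
; Tick scales the planet by mouse distance, snapping near unit scale, until right mouse or Space ends creation and returns control.
; The planet is serialized as editor-style actor copy-paste text and appended to the helper's master string.
; Undo/Redo teleport the planet far away or back and edit that string.
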(event Custom|TakeControl
  (params (Helper :type BP%20Level%20Design%20Helper%20Object%20Reference))
  (Variables|Default|SetLevelDesignHelper Helper)
  (Input|DisableInput Helper (Game|GetPlayerController 0))
  (CallFunction|StartCreation))

(event Custom|EndCreation
  (Actor|Tick|SetActorTickEnabled false)
  (CallFunction|BuildString)
  (CallFunction|Do (Variables|/Game/Blueprints/BP_LevelDesignHelper.BP_LevelDesignHelper_C|GetTheOneTrueString (Variables|Default|GetLevelDesignHelper)))
  (Default|TakeBackControl (Variables|Default|GetLevelDesignHelper) self)
  (CallFunction|UpdateUICurrentMode "Placement"))

(event Custom|StartCreation
  (bind _returnvalue (Game|SpawnActorfromClass "/Game/Blueprints/PlatformerLogic/Superclassi/BP_BasePlanet.BP_BasePlanet_C" (Math|Transform|MakeTransform (CallFunction|GetPlanetLocation) "0, 0, 0" "1,1,1") "AlwaysSpawn" 0 0))
  (Variables|Default|SetMyPlanet _returnvalue)
  (CallFunction|UpdateUICurrentMode "Scaling"))

(event EventTick
  (params (DeltaSeconds :type Float%20%28single-precision%29))
  (CallFunction|UpdatePlanetScale))

(event Input|MouseEvents|RightMouseButton
  (params (Key :type Key%20Structure :default "AnyKey"))
  (:Pressed
    (CallFunction|NextStep))
  (:Released
    (Utilities|FlowControl|DoOnce false
      (:Completed
        (CallFunction|NextStep)))))

(event Input|KeyboardEvents|SpaceBar
  (params (Key :type Key%20Structure :default "AnyKey"))
  (:Pressed
    (CallFunction|NextStep)))

(fn ConstructionScript)

(fn Undo
  (params (The%20One%20True%20String :type String%20%28by%20ref%29))
  (Transformation|AddActorWorldOffset (Variables|Default|GetMyPlanet) "0, 0,100000.000000" false true)
  (|SetBy-RefVar The%20One%20True%20String (Utilities|String|Replace The%20One%20True%20String (Variables|Default|GetMyStringPiece))))

(fn Do
  (params (The%20One%20True%20String :type String%20%28by%20ref%29))
  (|SetBy-RefVar The%20One%20True%20String (Utilities|String|Append The%20One%20True%20String (Variables|Default|GetMyStringPiece))))

(fn NextStep
  (CallFunction|EndCreation)
  (return true))

(fn UpdatePlanetScale
  (bind _returnvalue (CallFunction|GetMouseDistancefromPlanet))
  (bind _returnvalue_2 (Math|Vector|MakeVector 1.0 1.0 1.0))
  (bind _myplanet (Variables|Default|GetMyPlanet))
  (bind _snappingtolerance (LocalVariables|GetSnappingTolerance))
  (bind _minimumscale (LocalVariables|GetMinimumScale))
  (bind _returnvalue_3 (* _returnvalue_2 _returnvalue))
  (bind _returnvalue_4 (+ _returnvalue_3 _minimumscale))
  (bind _returnvalue_5 (Math|Vector|Equal(Vector) _returnvalue_4 "1.000000,1.000000,1.000000" _snappingtolerance))
  (bind _returnvalue_6 (Math|Vector|SelectVector "1.000000,1.000000,1.000000" _returnvalue_4 _returnvalue_5))
  (Transformation|SetActorScale3D _myplanet _returnvalue_6)
  (Default|ConstructFunction _myplanet)
  (return _returnvalue_6))

(fn BuildString
  (bind _myplanet (Variables|Default|GetMyPlanet))
  (bind _myplanet_2 (Variables|Default|GetMyPlanet))
  (bind _returnvalue (Transformation|GetActorLocation _myplanet_2))
  (bind _returnvalue_2 (Transformation|GetActorScale3D _myplanet))
  (bind (_x _y _z) (Math|Vector|BreakVector _returnvalue_2))
  (bind (_x_2 _y_2 _z_2) (Math|Vector|BreakVector _returnvalue))
  (Variables|Default|SetMyStringPiece " 
      Begin Actor Class=/Game/Blueprints/PlatformerLogic/Superclassi/BP_BasePlanet.BP_BasePlanet_C Name=TestPlanet30 Archetype=/Game/Blueprints/PlatformerLogic/Superclassi/BP_BasePlanet.BP_BasePlanet_C'/Game/Blueprints/PlatformerLogic/Superclassi/BP_BasePlanet.Default__BP_BasePlanet_C' 
         Begin Object Class=/Script/Engine.StaticMeshComponent Name=\"PlanetVisual\" Archetype=StaticMeshComponent'/Game/Blueprints/PlatformerLogic/Superclassi/BP_BasePlanet.BP_BasePlanet_C:PlanetVisual_GEN_VARIABLE' 
         End Object 
         Begin Object Class=/Script/Engine.SceneComponent Name=\"PlanetRotationPivot\" Archetype=SceneComponent'/Game/Blueprints/PlatformerLogic/Superclassi/BP_BasePlanet.BP_BasePlanet_C:PlanetRotationPivot_GEN_VARIABLE' 
         End Object 
         Begin Object Class=/Script/Engine.SphereComponent Name=\"PlanetSurfaceCollision\" Archetype=SphereComponent'/Game/Blueprints/PlatformerLogic/Superclassi/BP_BasePlanet.BP_BasePlanet_C:PlanetSurfaceCollision_GEN_VARIABLE' 
         End Object 
         Begin Object Name=\"PlanetVisual\" 
            AttachParent=PlanetSurfaceCollision 
            bNetAddressable=True 
            CreationMethod=SimpleConstructionScript 
         End Object 
         Begin Object Name=\"PlanetRotationPivot\" 
            AttachParent=PlanetSurfaceCollision 
            bNetAddressable=True 
            CreationMethod=SimpleConstructionScript 
         End Object 
         Begin Object Name=\"PlanetSurfaceCollision\" 
            RelativeLocation=(")
  (Variables|Default|SetMyStringPiece (Utilities|String|Append (Variables|Default|GetMyStringPiece) "X=" (Utilities|String|ToString(Float) _x_2) "," "Y=" (Utilities|String|ToString(Float) _y_2) "," "Z=" (Utilities|String|ToString(Float) _z_2)))
  (Variables|Default|SetMyStringPiece (Utilities|String|Append (Variables|Default|GetMyStringPiece) ") 
            RelativeScale3D=("))
  (Variables|Default|SetMyStringPiece (Utilities|String|Append (Variables|Default|GetMyStringPiece) "X=" (Utilities|String|ToString(Float) _x) "," "Y=" (Utilities|String|ToString(Float) _y) "," "Z=" (Utilities|String|ToString(Float) _z)))
  (bind _output_get (Variables|Default|SetMyStringPiece (Utilities|String|Append (Variables|Default|GetMyStringPiece) ") 
            bNetAddressable=True 
            CreationMethod=SimpleConstructionScript 
            UCSModifiedProperties(0)=(MemberParent=Class'/Script/Engine.SceneComponent',MemberName=\"RelativeLocation\") 
            UCSModifiedProperties(2)=(MemberParent=Class'/Script/Engine.SceneComponent',MemberName=\"RelativeScale3D\") 
         End Object 
         PlanetVisual=PlanetVisual 
         PlanetSurfaceCollision=PlanetSurfaceCollision 
         PlanetRotationPivot=PlanetRotationPivot 
         RootComponent=PlanetSurfaceCollision 
         ActorLabel=\"TestPlanet30\" 
      End Actor 
")))
  (return _output_get))

(fn GetPlanetLocation
  (bind _returnvalue (Game|GetPlayerController 0))
  (bind _worldlocation (Game|Player|ConvertMouseLocationToWorldSpace _returnvalue))
  (bind (_x _y _z) (Math|Vector|BreakVector _worldlocation))
  (return (Math|Vector|MakeVector _x 0.0 _z)))

(fn GetMouseDistancefromPlanet
  (bind _returnvalue (Game|GetPlayerController 0))
  (bind _worldlocation (Game|Player|ConvertMouseLocationToWorldSpace _returnvalue))
  (bind (_x _y _z) (Math|Vector|BreakVector _worldlocation))
  (return (* (Math|Vector|VectorLength (- (Transformation|GetActorLocation (Variables|Default|GetMyPlanet)) (Math|Vector|MakeVector _x 0.0 _z))) 0.01)))

(fn UpdateUICurrentMode
  (params (NewText :type Text))
  (Default|UpdateCurrentMode (Variables|/Game/Blueprints/BP_LevelDesignHelper.BP_LevelDesignHelper_C|GetUIWidget (Variables|Default|GetLevelDesignHelper)) NewText)
  (return true))

(fn AppendtoMyStringPiece
  (params (StringToAppend :type String))
  (bind _output_get (Variables|Default|SetMyStringPiece (Utilities|String|Append (Variables|Default|GetMyStringPiece) StringToAppend)))
  (return _output_get))

(fn Redo
  (params (The%20One%20True%20String :type String%20%28by%20ref%29))
  (Transformation|AddActorWorldOffset (Variables|Default|GetMyPlanet) "0, 0,-100000.000000" false true)
  (|SetBy-RefVar The%20One%20True%20String (Utilities|String|Append The%20One%20True%20String (Variables|Default|GetMyStringPiece))))