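; In-game creator that spawns a BP_ExplodingPlanet and lets the player shape it with the mouse in stages.
; NextStep advances a counter through scaling, detection radius, explosion radius and placement, updating the UI mode label.
; Tick applies the current stage, refreshing the planet's visible radius previews, then calls EndCreation at placement.
; BuildString serializes the planet as Unreal actor copy-paste text, inserting its location, scale and radii into a hard-coded template.
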(event EventBeginPlay)

(event Collision|EventActorBeginOverlap
  (params (OtherActor :type Actor%20Object%20Reference)))

(event EventTick
  (params (DeltaSeconds :type Float%20%28single-precision%29))
  (bind _myexplodingplanet (Variables|Default|GetMyExplodingPlanet))
  (switch int (Variables|Default|GetDerp)
    (:0
      (CallFunction|UpdatePlanetScale))
    (:1
      (Variables|/Game/Blueprints/PlatformerLogic/Superclassi/BP_BasePlanetDetecting.BP_BasePlanetDetecting_C|SetDetectionRadius _myexplodingplanet (* (CallFunction|GetMouseDistancefromPlanet) 1e+02))
      (Default|ConstructFunction _myexplodingplanet))
    (:2
      (Variables|/Game/Blueprints/PlatformerLogic/BP_ExplodingPlanet.BP_ExplodingPlanet_C|SetExplosionRadius (Variables|Default|GetMyExplodingPlanet) (* (CallFunction|GetMouseDistancefromPlanet) 2.0))
      (Default|ConstructFunction (Variables|Default|GetMyExplodingPlanet)))
    (:3
      (CallFunction|EndCreation))))

(event EventStartCreation
  (bind _returnvalue (Game|SpawnActorfromClass "/Game/Blueprints/PlatformerLogic/BP_ExplodingPlanet.BP_ExplodingPlanet_C" (Math|Transform|MakeTransform (CallFunction|GetPlanetLocation) "0, 0, 0" "1,1,1") "Undefined" 0 0))
  (Variables|Default|SetMyPlanet _returnvalue)
  (bind _output_get (Variables|Default|SetMyExplodingPlanet _returnvalue))
  (Development|SetHiddeninGame (Variables|/Game/Blueprints/PlatformerLogic/BP_ExplodingPlanet.BP_ExplodingPlanet_C|GetExplosionPreview _output_get) false true)
  (CallFunction|UpdateUICurrentMode "Scaling"))

(fn ConstructionScript
  (|CallParentFunction))

(fn NextStep
  (bind _result (Math|Integer|IncrementInt (Variables|Default|GetDerp))
    (:%20%20
      (switch int _result
        (:1
          (CallFunction|UpdateUICurrentMode "Detection Radius"))
        (:2
          (CallFunction|UpdateUICurrentMode "Explosion Radius"))
        (:3
          (CallFunction|UpdateUICurrentMode "Placement")
          (return true)))
      (return false))))

(fn BuildString
  (bind _myplanet (Variables|Default|GetMyPlanet))
  (bind _myplanet_2 (Variables|Default|GetMyPlanet))
  (bind _returnvalue (Transformation|GetActorLocation _myplanet_2))
  (bind _returnvalue_2 (Transformation|GetActorScale3D _myplanet))
  (bind (_x _y _z) (Math|Vector|BreakVector _returnvalue_2))
  (bind (_x_2 _y_2 _z_2) (Math|Vector|BreakVector _returnvalue))
  (Variables|Default|SetMyStringPiece " 
      Begin Actor Class=/Game/Blueprints/PlatformerLogic/BP_ExplodingPlanet.BP_ExplodingPlanet_C Name=BP_ExplodingPlanet_262 Archetype=/Game/Blueprints/PlatformerLogic/BP_ExplodingPlanet.BP_ExplodingPlanet_C'/Game/Blueprints/PlatformerLogic/BP_ExplodingPlanet.Default__BP_ExplodingPlanet_C' 
         Begin Object Class=/Script/Engine.TimelineComponent Name=\"ExplosionBuildup\" 
         End Object 
         Begin Object Class=/Script/Engine.StaticMeshComponent Name=\"ExplosionPreview\" Archetype=StaticMeshComponent'/Game/Blueprints/PlatformerLogic/BP_ExplodingPlanet.BP_ExplodingPlanet_C:ExplosionPreview_GEN_VARIABLE' 
         End Object 
         Begin Object Class=/Script/Engine.SphereComponent Name=\"DetectionCollision\" Archetype=SphereComponent'/Game/Blueprints/PlatformerLogic/Superclassi/BP_BasePlanetDetecting.BP_BasePlanetDetecting_C:DetectionCollision_GEN_VARIABLE' 
            Begin Object Class=/Script/Engine.BodySetup Name=\"BodySetup_27\" 
            End Object 
         End Object 
         Begin Object Class=/Script/Engine.StaticMeshComponent Name=\"PlanetVisual\" Archetype=StaticMeshComponent'/Game/Blueprints/PlatformerLogic/BP_ExplodingPlanet.BP_ExplodingPlanet_C:PlanetVisual_GEN_VARIABLE' 
         End Object 
         Begin Object Class=/Script/Engine.SceneComponent Name=\"PlanetRotationPivot\" Archetype=SceneComponent'/Game/Blueprints/PlatformerLogic/Superclassi/BP_BasePlanet.BP_BasePlanet_C:PlanetRotationPivot_GEN_VARIABLE' 
         End Object 
         Begin Object Class=/Script/Engine.SphereComponent Name=\"PlanetSurfaceCollision\" Archetype=SphereComponent'/Game/Blueprints/PlatformerLogic/BP_ExplodingPlanet.BP_ExplodingPlanet_C:PlanetSurfaceCollision_GEN_VARIABLE' 
         End Object 
         Begin Object Name=\"ExplosionBuildup\" 
            TheTimeline=(LengthMode=TL_TimelineLength,Length=1.000000,InterpFloats=((FloatCurve=CurveFloat'/Game/Blueprints/PlatformerLogic/BP_ExplodingPlanet.BP_ExplodingPlanet_C:CurveFloat_0',TrackName=\"ZeroOne\",FloatPropertyName=\"ExplosionBuildup_ZeroOne_E87526F54FC7D93BE0A57090A5693450\")),TimelinePostUpdateFunc=BP_ExplodingPlanet_262.ExplosionBuildup__UpdateFunc,TimelineFinishedFunc=BP_ExplodingPlanet_262.ExplosionBuildup__FinishedFunc,PropertySetObject=BP_ExplodingPlanet_C'BP_ExplodingPlanet_262',DirectionPropertyName=\"ExplosionBuildup__Direction_E87526F54FC7D93BE0A57090A5693450\") 
            bNetAddressable=True 
            CreationMethod=UserConstructionScript 
         End Object 
         Begin Object Name=\"ExplosionPreview\" 
            AttachParent=PlanetSurfaceCollision 
            RelativeScale3D=(X=4.396209,Y=4.396209,Z=4.396209) 
            bNetAddressable=True 
            CreationMethod=SimpleConstructionScript 
            UCSModifiedProperties(0)=(MemberParent=Class'/Script/Engine.SceneComponent',MemberName=\"RelativeScale3D\") 
         End Object 
         Begin Object Name=\"DetectionCollision\" 
            Begin Object Name=\"BodySetup_27\" 
               AggGeom=(SphereElems=((TM=(XPlane=(W=0.000000,X=-0.000000,Y=0.000000,Z=0.000000),YPlane=(W=0.000000,X=0.000000,Y=0.000000,Z=0.000000),ZPlane=(W=0.000000,X=0.000000,Y=0.000000,Z=24660167078163148653226622976.000000),WPlane=(W=0.000000,X=24659033710207259938375335936.000000,Y=0.000000,Z=0.003610)),Radius=155.318390))) 
               CollisionTraceFlag=CTF_UseSimpleAsComplex 
            End Object 
            SphereRadius=155.318390 
            AttachParent=PlanetSurfaceCollision 
            bNetAddressable=True 
            CreationMethod=SimpleConstructionScript 
            UCSModifiedProperties(0)=(MemberParent=Class'/Script/Engine.SphereComponent',MemberName=\"SphereRadius\") 
         End Object 
         Begin Object Name=\"PlanetVisual\" 
            AttachParent=PlanetSurfaceCollision 
            bNetAddressable=True 
            CreationMethod=SimpleConstructionScript 
         End Object 
         Begin Object Name=\"PlanetRotationPivot\" 
            AttachParent=PlanetSurfaceCollision 
            bNetAddressable=True 
            CreationMethod=SimpleConstructionScript 
         End Object 
         Begin Object Name=\"PlanetSurfaceCollision\" 
            RelativeLocation=(")
  (Variables|Default|SetMyStringPiece (Utilities|String|Append (Variables|Default|GetMyStringPiece) "X=" (Utilities|String|ToString(Float) _x_2) "," "Y=" (Utilities|String|ToString(Float) _y_2) "," "Z=" (Utilities|String|ToString(Float) _z_2)))
  (Variables|Default|SetMyStringPiece (Utilities|String|Append (Variables|Default|GetMyStringPiece) ") 
            RelativeScale3D=("))
  (Variables|Default|SetMyStringPiece (Utilities|String|Append (Variables|Default|GetMyStringPiece) "X=" (Utilities|String|ToString(Float) _x) "," "Y=" (Utilities|String|ToString(Float) _y) "," "Z=" (Utilities|String|ToString(Float) _z)))
  (Variables|Default|SetMyStringPiece (Utilities|String|Append (Variables|Default|GetMyStringPiece) ") 
            bNetAddressable=True 
            CreationMethod=SimpleConstructionScript 
            UCSModifiedProperties(0)=(MemberParent=Class'/Script/Engine.SceneComponent',MemberName=\"RelativeLocation\") 
            UCSModifiedProperties(1)=(MemberParent=Class'/Script/Engine.SceneComponent',MemberName=\"RelativeScale3D\") 
         End Object 
         ExplosionPreview=ExplosionPreview 
         ExplosionBuildup=TimelineComponent'ExplosionBuildup' 
         ExplosionRadius="))
  (CallFunction|AppendtoMyStringPiece (Utilities|String|ToString(Float) (Variables|/Game/Blueprints/PlatformerLogic/BP_ExplodingPlanet.BP_ExplodingPlanet_C|GetExplosionRadius (Variables|Default|GetMyExplodingPlanet))))
  (CallFunction|AppendtoMyStringPiece " 
         ExplosionIntensity=1855.234497 
         DetectionCollision=DetectionCollision 
         DetectionRadius=")
  (CallFunction|AppendtoMyStringPiece (Utilities|String|ToString(Float) (Variables|/Game/Blueprints/PlatformerLogic/Superclassi/BP_BasePlanetDetecting.BP_BasePlanetDetecting_C|GetDetectionRadius (Variables|Default|GetMyExplodingPlanet))))
  (CallFunction|AppendtoMyStringPiece " 
         PlanetVisual=PlanetVisual 
         PlanetSurfaceCollision=PlanetSurfaceCollision 
         PlanetRotationPivot=PlanetRotationPivot 
         DeathTime=1.588406 
         RootComponent=PlanetSurfaceCollision 
         ActorLabel=\"BP_ExplodingPlanet\" 
      End Actor 
")
  (return (Variables|Default|GetMyStringPiece)))