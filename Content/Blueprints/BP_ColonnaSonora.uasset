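; BP_ColonnaSonora is a soundtrack actor that starts the music and sets a background when play begins.
; On BeginPlay it plays a random track from the Canzoni array as a non-spatial 2D sound at slightly reduced volume.
; It then finds all BP_Tumy actors and calls ModificaSprite with BackgroundSize and BackgroundImage with NuovoBackground on them.
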(event EventBeginPlay
  (bind _canzoni (Variables|Default|Getcanzoni))
  (Utilities|FlowControl|Sequence
    (:then_0
      (Audio|PlaySound2D (Utilities|Array|Get(acopy) _canzoni (Math|Random|RandomInteger (Utilities|Array|Length _canzoni))) 0.8))
    (:then_1
      (bind _outactors (Actor|GetAllActorsOfClass "/Game/Blueprints/Tumy/BP_Tumy.BP_Tumy_C"))
      (Default|ModificaSprite _outactors (Variables|Default|Getbackground%20size))
      (Default|BackgroundImage _outactors (Variables|Default|Getnuovo%20background)))))

(event EventActorBeginOverlap
  (params (OtherActor :type Actor%20Object%20Reference)))

(event EventTick
  (params (DeltaSeconds :type Float%20%28single-precision%29)))

(fn ConstructionScript)