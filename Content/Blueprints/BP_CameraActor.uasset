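; BP_CameraActor is a side-on follow camera that becomes the first player controller's view target on BeginPlay.
; Every Tick it teleports to the Target actor's X and Z while holding Y at a hard-coded depth, with no smoothing.
; The construction script sets a fixed rotation and a different, farther Y offset, which the first Tick overrides.
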(event EventBeginPlay
  (Game|Player|SetViewTargetwithBlend (Game|GetPlayerController 0) self 0.0 "VTBlend_Linear" 0.0 false))

(event Collision|EventActorBeginOverlap
  (params (OtherActor :type Actor%20Object%20Reference)))

(event EventTick
  (params (DeltaSeconds :type Float%20%28single-precision%29))
  (bind _target (Variables|Default|GetTarget))
  (bind _returnvalue (Transformation|GetActorLocation _target))
  (Transformation|SetActorLocation (Math|Vector|MakeVector (.x _returnvalue) 999.0 (.z _returnvalue)) false true))

(fn ConstructionScript
  (bind _returnvalue (Transformation|GetActorLocation))
  (Transformation|SetActorLocation (Math|Vector|MakeVector (.x _returnvalue) 4e+03 (.z _returnvalue)) false false)
  (Transformation|SetActorRotation "0,-90.000000, 0"))