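; In-game level design tool that places platforms during play and exports the layout to the OS clipboard as Unreal map paste text.
; Mouse input pauses via slomo, pans and zooms the orthographic camera, and spawns the Tab-selected creator, which borrows input until it hands back control.
; A stored creator array drives undo/redo on one map string, whose closing tags are stripped and re-appended around edits.
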(event Custom|Take%20Back%20Control
  (params (ActorCreator :type BP%20Level%20Design%20Actor%20Creator%20Object%20Reference))
  (Input|DisableInput ActorCreator (Game|GetPlayerController 0))
  (Input|EnableInput (Game|GetPlayerController 0))
  (CallFunction|CloseSuperFantasticString))

(event EventBeginPlay
  (Utilities|DeactivationCriteria
    (:Go
      (Development|PrintString "LEVEL DESIGN HELPER ACTIVE" true true "(R=0.000000,G=0.000000,B=1.000000,A=1.000000)" 1e+01)
      (Variables|/Script/Engine.PlayerController|SetbShowMouseCursor (Game|GetPlayerController 0) true)
      (bind _outactors (Actor|GetAllActorsOfClass "/Game/Blueprints/BP_CameraActor.BP_CameraActor_C"))
      (Variables|Default|SetCameraActor (Utilities|Array|Get(acopy) _outactors))
      (Game|SpawnActorfromClass "/Game/Blueprints/BP_LevelDesignToggler.BP_LevelDesignToggler_C" (Math|Transform|MakeTransform "0, 0, 0" "0, 0, 0" "1,1,1") "AlwaysSpawn" 0 self 0)
      (bind _returnvalue (UserInterface|CreateWidget "/Game/Widgets/LevelEditor/WBP_LevelEditorBase.WBP_LevelEditorBase_C"))
      (Variables|Default|SetUIWidget _returnvalue)
      (UserInterface|Viewport|AddtoPlayerScreen _returnvalue))))

(event EventTick
  (params (DeltaSeconds :type Float%20%28single-precision%29)))

(event Input|KeyboardEvents|Tab
  (params (Key :type Key%20Structure :default "AnyKey"))
  (:Pressed
    (CallFunction|ScrollPlatType)))

(event Input|KeyboardEvents|CtrlShiftZ
  (params (Key :type Key%20Structure :default "AnyKey"))
  (:Pressed
    (Math|Integer|IncrementInt (Variables|Default|GetSpawnedCreatorsIndex)
      (:%20%20
        (if (< (- (Variables|Default|GetSpawnedCreatorsIndex) 1) (Utilities|Array|Length (Variables|Default|GetSpawnedCreators)))
          (CallFunction|OpenSuperFantasticString)
          (Default|Redo (Utilities|Array|Get(acopy) (Variables|Default|GetSpawnedCreators) (- (Variables|Default|GetSpawnedCreatorsIndex) 1)) (Variables|Default|GetTheOneTrueString))
          (CallFunction|CloseSuperFantasticString)
          (else
            (Math|Integer|DecrementInt (Variables|Default|GetSpawnedCreatorsIndex))))))))

(event Input|KeyboardEvents|CtrlZ
  (params (Key :type Key%20Structure :default "AnyKey"))
  (:Pressed
    (if (> (Variables|Default|GetSpawnedCreatorsIndex) 0)
      (Default|Undo (Utilities|Array|Get(acopy) (Variables|Default|GetSpawnedCreators) (- (Variables|Default|GetSpawnedCreatorsIndex) 1)) (Variables|Default|GetTheOneTrueString))
      (Math|Integer|DecrementInt (Variables|Default|GetSpawnedCreatorsIndex)
        (:%20%20
          (Class|VictoryBPFunctionLibrary|VictorySaveStringtoOSClipboard (Variables|Default|GetTheOneTrueString)))))))

(event Input|MouseEvents|LeftMouseButton
  (params (Key :type Key%20Structure :default "AnyKey"))
  (bind _cameraactor (Variables|Default|GetCameraActor))
  (bind _camera1 (Variables|/Game/Blueprints/BP_CameraActor.BP_CameraActor_C|GetCamera1 _cameraactor))
  (:Pressed
    (Utilities|LockInputwithKey (Variables|InputLockSystem|GetCameraMovementLockString))
    (Utilities|StopGame)
    (bind _returnvalue (AddComponent|AddBPLevelDesignCameraMover))
    (Default|Initialize _returnvalue _camera1)
    (Variables|MovingtheCamera|SetStoredCamPosition (Transformation|GetWorldLocation _camera1)))
  (:Released
    (Utilities|UnlockInputwithKey (Variables|InputLockSystem|GetCameraMovementLockString)
      (:Resolved
        (Components|DestroyComponent _returnvalue)))))

(event Input|MouseEvents|MouseWheelDown
  (params (Key :type Key%20Structure :default "AnyKey"))
  (bind _cameraactor (Variables|Default|GetCameraActor))
  (bind _camera1 (Variables|/Game/Blueprints/BP_CameraActor.BP_CameraActor_C|GetCamera1 _cameraactor))
  (bind _orthowidth (Variables|/Script/Engine.CameraComponent|GetOrthoWidth _camera1))
  (:Pressed
    (Class|CameraComponent|SetOrthoWidth _camera1 (* _orthowidth 1.1))
    (Development|PrintString (Utilities|String|ToString(Float) _orthowidth))))

(event Input|MouseEvents|MouseWheelUp
  (params (Key :type Key%20Structure :default "AnyKey"))
  (bind _cameraactor (Variables|Default|GetCameraActor))
  (bind _camera1 (Variables|/Game/Blueprints/BP_CameraActor.BP_CameraActor_C|GetCamera1 _cameraactor))
  (:Pressed
    (Class|CameraComponent|SetOrthoWidth _camera1 (* (Variables|/Script/Engine.CameraComponent|GetOrthoWidth _camera1) 0.9))
    (Development|PrintString (Utilities|String|ToString(Float) (Variables|/Script/Engine.CameraComponent|GetOrthoWidth (Variables|/Game/Blueprints/BP_CameraActor.BP_CameraActor_C|GetCamera1 (Variables|Default|GetCameraActor)))))))

(event Input|MouseEvents|MiddleMouseButton
  (params (Key :type Key%20Structure :default "AnyKey"))
  (:Pressed
    (Utilities|InputLockSwitch
      (:Unlocked
        (if (Variables|Default|GetIsPaused)
          (Utilities|ResumeGame)
          (else
            (Utilities|StopGame)))))))

(event Input|MouseEvents|RightMouseButton
  (params (Key :type Key%20Structure :default "AnyKey"))
  (:Pressed
    (Utilities|InputLockSwitch
      (:Unlocked
        (Utilities|FlowControl|Sequence
          (:then_1
            (CallFunction|OpenSuperFantasticString)
            (Utilities|StopGame)
            (Input|DisableInput (Game|GetPlayerController 0))
            (bind _level_design_actor_creator (CallFunction|CreateCreator))
            (Default|TakeControl _level_design_actor_creator self)))))))

(event Input|KeyboardEvents|7
  (params (Key :type Key%20Structure :default "AnyKey")))

(fn ConstructionScript)

(fn OpenSuperFantasticString
  (if (== (Utilities|String|Len (Variables|Default|GetTheOneTrueString)) 0)
    (Variables|Default|SetTheOneTrueString "Begin Map 
   Begin Level")
    (else
      (Variables|Default|SetTheOneTrueString (Utilities|String|Replace (Variables|Default|GetTheOneTrueString) "   End Level 
Begin Surface 
End Surface 
End Map 
" "" "CaseSensitive")))))

(fn CreateCreator
  (bind _returnvalue (Game|SpawnActorfromClass (.creator (Utilities|Array|Get(acopy) (Variables|Default|GetCreators) (Variables|Default|GetCurrentPlatformTypeIndex))) (Math|Transform|MakeTransform "0, 0, 0" "0, 0, 0" "1,1,1") "AlwaysSpawn" 0 0))
  (Utilities|Array|SetArrayElem (Variables|Default|GetSpawnedCreators) (Variables|Default|GetSpawnedCreatorsIndex) _returnvalue true)
  (Math|Integer|IncrementInt (Variables|Default|GetSpawnedCreatorsIndex)
    (:%20%20
      (return _returnvalue))))

(fn ScrollPlatType
  (Math|Integer|IncrementInt (Variables|Default|GetCurrentPlatformTypeIndex)
    (:%20%20
      (if (== (Utilities|Array|Length (Variables|Default|GetCreators)) (Variables|Default|GetCurrentPlatformTypeIndex))
        (Variables|Default|SetCurrentPlatformTypeIndex 0))
      (Default|UpdateCurrentPlatform (Variables|Default|GetUIWidget) (Utilities|Text|ToText(Name) (.name (Utilities|Array|Get(acopy) (Variables|Default|GetCreators) (Variables|Default|GetCurrentPlatformTypeIndex)))))
      (return))))

(fn CloseSuperFantasticString
  (bind _output_get (Variables|Default|SetTheOneTrueString (Utilities|String|Append (Variables|Default|GetTheOneTrueString) "   End Level 
Begin Surface 
End Surface 
End Map 
")))
  (Class|VictoryBPFunctionLibrary|VictorySaveStringtoOSClipboard _output_get))