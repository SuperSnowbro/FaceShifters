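; Level design camera mover that pans a camera component on the X/Z plane by following mouse movement.
; Initialize stores the camera component, its world position and the DPI-scaled mouse position as anchors.
; Each Tick adds the mouse offset from that anchor, opposite to horizontal movement, to the stored position.
; CameraMovementSensitivity multiplies that whole sum, not just the offset, before the camera teleports there.
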(event Custom|Initialize
  (params (CameraComponent :type Camera%20Component%20Object%20Reference))
  (bind _returnvalue (Game|GetPlayerController 0))
  (bind (_locationx _locationy) (Class|WidgetLayoutLibrary|GetMousePositionScaledbyDPI _returnvalue))
  (Variables|Default|SetCameraComponent CameraComponent)
  (Variables|Default|SetStoredMousePosition (Math|Vector2D|MakeVector2D _locationx _locationy))
  (Variables|Default|SetStoredCamPosition (Transformation|GetWorldLocation (Variables|Default|GetCameraComponent))))

(event EventTick
  (params (DeltaSeconds :type Float%20%28single-precision%29))
  (bind _returnvalue (Game|GetPlayerController 0))
  (bind _storedmouseposition (Variables|Default|GetStoredMousePosition))
  (bind (_locationx _locationy) (Class|WidgetLayoutLibrary|GetMousePositionScaledbyDPI _returnvalue))
  (bind _returnvalue_2 (Math|Vector2D|MakeVector2D _locationx _locationy))
  (bind _returnvalue_3 (- _storedmouseposition _returnvalue_2))
  (Transformation|SetWorldLocation (Variables|Default|GetCameraComponent) (* (+ (Variables|Default|GetStoredCamPosition) (Math|Vector|MakeVector (.x _returnvalue_3) 0.0 (* (.y _returnvalue_3) -1.0))) (Variables|Default|GetCameraMovementSensitivity)) false true))